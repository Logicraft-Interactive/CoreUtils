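; BP_TestBlueprintPool is a debug test harness for the object pool subsystem.
; On BeginPlay it creates a pool of BP_PoolableTest from the DA_BasicPool data asset.
; A debug R key press spawns a pooled actor at a random offset around itself and tracks it in an array.
; A debug T key press returns a random tracked actor to the pool and removes it from the array.
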(event EventBeginPlay
  (bind _returnvalue (Class|PoolSubsystem|CreatePoolfromDataAsset (Subsystems|GetPoolSubsystem) "/Game/Pool/BP_PoolableTest.BP_PoolableTest_C" "/Game/Pool/DA_BasicPool.DA_BasicPool"))
  (Variables|Default|SetPool%20Object _returnvalue))

(event Input|KeyboardEvents|DebugKeyR
  (params (Key :type Key%20Structure :default "None") (ActionValue :type Input%20Action%20Value%20Structure))
  (bind _returnvalue (Transformation|GetActorTransform))
  (:Pressed
    (bind _returnvalue_2 (Class|PoolObject|SpawnfromPool (Variables|Default|GetPool%20Object) (Math|Transform|MakeTransform (+ (* (Math|Random|RandomUnitVector) 5e+02) (.location _returnvalue)) (.rotation _returnvalue) (.scale _returnvalue))))
    (Utilities|Array|Add (Variables|Default|GetActors) _returnvalue_2)))

(event Input|KeyboardEvents|DebugKeyT
  (params (Key :type Key%20Structure :default "None") (ActionValue :type Input%20Action%20Value%20Structure))
  (bind _actors (Variables|Default|GetActors))
  (:Pressed
    (bind _output_get (Variables|Default|SetNewVar (Utilities|Array|Get(acopy) _actors (Math|Random|RandomIntegerinRange 0 (- (Utilities|Array|Length _actors) 1)))))
    (Class|PoolObject|ReturntoPool (Variables|Default|GetPool%20Object) _output_get)
    (Utilities|Array|RemoveItem (Variables|Default|GetActors) _output_get)))

(fn ConstructionScript)